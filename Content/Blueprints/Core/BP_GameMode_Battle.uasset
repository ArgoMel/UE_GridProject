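; Battle game mode that spawns the enemy and friendly monsters from save games when play begins.
; The enemy's class and stats come from the enemy monster save; the friendly monster is the first entry in the party save's map of classes to stats.
; Each spawns at the location of the first actor carrying its side's spawn tag, then receives its saved stats.
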(event EventBeginPlay
  (Utilities|FlowControl|Sequence
    (:then_0
      (bind _returnvalue (SaveGame|LoadGamefromSlot "EnemyMonsterSave" 101))
      (bind _aspmonster_save (Utilities|Casting|CastToPMonsterSave _returnvalue))
      ;[1 0 0] Enemy Monster Spawn
      (bind _outactors (Actor|GetAllActorswithTag "EnemyMonsterSpawn"))
      (bind _returnvalue_2 (Game|SpawnActorfromClass (Variables|/Script/Pixel.PMonsterSave|GetMonsterReference _aspmonster_save) (Math|Conversions|ToTransform(Vector) (Transformation|GetActorLocation (Utilities|Array|Get(acopy) _outactors))) "AdjustIfPossibleButAlwaysSpawn" 0 0))
      (Variables|/Script/Pixel.PMonsterStats|SetMonsterStats (Variables|/Script/Pixel.PMonster|GetMonsterStats _returnvalue_2) (Variables|/Script/Pixel.PMonsterSave|GetMonsterStats _aspmonster_save)))
    (:then_1
      (bind _returnvalue_3 (SaveGame|LoadGamefromSlot "PlayerMonsterPartySave" 200))
      (bind _aspmonster_party_save (Utilities|Casting|CastToPMonsterPartySave _returnvalue_3))
      (bind _keys (Utilities|Map|Keys (Variables|/Script/Pixel.PMonsterPartySave|GetMonsterParty _aspmonster_party_save)))
      (bind _values (Utilities|Map|Values (Variables|/Script/Pixel.PMonsterPartySave|GetMonsterParty _aspmonster_party_save)))
      ;[0.07021 1 0] Friendly Monster Spawn
      (bind _outactors_2 (Actor|GetAllActorswithTag "FriendlyMonsterSpawn"))
      (bind _returnvalue_4 (Game|SpawnActorfromClass (Utilities|Array|Get(acopy) _keys) (Math|Conversions|ToTransform(Vector) (Transformation|GetActorLocation (Utilities|Array|Get(acopy) _outactors_2))) "AdjustIfPossibleButAlwaysSpawn" 0 0))
      (Variables|/Script/Pixel.PMonsterStats|SetMonsterStats (Variables|/Script/Pixel.PMonster|GetMonsterStats _returnvalue_4) (Utilities|Array|Get(acopy) _values)))))

(fn ConstructionScript)