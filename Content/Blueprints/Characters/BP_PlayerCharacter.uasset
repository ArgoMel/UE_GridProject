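; BP_PlayerCharacter is the player-controlled character, handling movement, look and jump input.
; When its TriggerSphere overlaps an actor that returns a valid GetMonsterMessage result, it passes its MonsterParty data to the Game Instance through SaveMonsterPartyMessage.
; The monster result only gates the save and is not passed on.
; GetPlayerCharacter simply returns the character itself.
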(event OnComponentBeginOverlap(TriggerSphere)
  (params (OverlappedComponent :type Primitive%20Component%20Object%20Reference) (OtherActor :type Actor%20Object%20Reference) (OtherComp :type Primitive%20Component%20Object%20Reference) (OtherBodyIndex :type Integer) (bFromSweep :type Boolean) (SweepResult :type Hit%20Result%20Structure%20%28by%20ref%29))
  (bind _monster (Class|IMonster|GetMonster(Message) OtherActor))
  (Utilities|IsValid _monster
    (:Is%20Valid
      (Class|PGameInstanceInterface|SaveMonsterParty(Message) (Game|GetGameInstance) (Variables|/Script/Pixel.PMonsterParty|GetMonsterParty (Variables|Default|GetMonster%20Party))))))

(event Input|ActionEvents|InputActionJump
  (params (Key :type Key%20Structure :default "None"))
  (:Pressed
    (Character|Jump)))

(event Input|AxisEvents|InputAxisForward
  (params (AxisValue :type Float%20%28single-precision%29))
  (Pawn|Input|AddMovementInput (Transformation|GetActorForwardVector) AxisValue false))

(event Input|AxisEvents|InputAxisRight
  (params (AxisValue :type Float%20%28single-precision%29))
  (Pawn|Input|AddMovementInput (Transformation|GetActorRightVector) AxisValue false))

(event Input|AxisEvents|InputAxisLookUp
  (params (AxisValue :type Float%20%28single-precision%29))
  (Pawn|Input|AddControllerPitchInput AxisValue))

(event Input|AxisEvents|InputAxisTurn
  (params (AxisValue :type Float%20%28single-precision%29))
  (Pawn|Input|AddControllerYawInput AxisValue))

(fn ConstructionScript)

(fn GetPlayerCharacter
  (return self))